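; BP_Hand is a left or right Oculus tracked hand that acts as a laser pointer for widget UI.
; The construction script sets motion source and hand mesh from the Hand variable; BeginPlay assigns a pointer index per hand.
; Each tick, high tracking confidence and a valid pointer pose move the spline and WidgetInteraction, stretching a spline-mesh beam to blocking hits, otherwise collapsing it.
; Press and Release events simulate left mouse clicks.
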(event Custom|Press
  (Class|WidgetInteractionComponent|PressPointerKey (Variables|Default|GetWidgetInteraction) "LeftMouseButton"))

(event Custom|Release
  (Class|WidgetInteractionComponent|ReleasePointerKey (Variables|Default|GetWidgetInteraction) "LeftMouseButton"))

(event EventTick
  (params (DeltaSeconds :type Float%20%28single-precision%29))
  (bind _returnvalue (Transformation|GetActorTransform))
  (bind _returnvalue_2 (CallFunction|GetOculusHandType))
  (bind _widgetinteraction (Variables|Default|GetWidgetInteraction))
  (bind _returnvalue_3 (Class|OculusInputFunctionLibrary|GetPointerPose _returnvalue_2))
  (bind _returnvalue_4 (Class|WidgetInteractionComponent|GetLastHitResult _widgetinteraction))
  (bind (_bblockinghit _binitialoverlap _time _distance _location) (Collision|BreakHitResult _returnvalue_4))
  (switch Utilities|FlowControl|Switch|SwitchonETrackingConfidence (Class|OculusInputFunctionLibrary|GetTrackingConfidence (CallFunction|GetOculusHandType))
    (:Low
      (CallFunction|CollapseSpline))
    (:High
      (if (Class|OculusInputFunctionLibrary|IsPointerPoseValid (CallFunction|GetOculusHandType))
        (Transformation|SetWorldLocationAndRotation (Variables|Default|GetSpline) (Math|Transform|TransformLocation _returnvalue (.location _returnvalue_3)) (Math|Transform|TransformRotation _returnvalue (.rotation _returnvalue_3)) false false)
        (if _bblockinghit
          (Spline|SetLocationatSplinePoint (Variables|Default|GetSpline) 1 _location "World" true)
          (CallFunction|UpdateSplineMesh)
          (else
            (CallFunction|CollapseSpline)))
        (else
          (CallFunction|CollapseSpline))))))

(event EventBeginPlay
  (bind _widgetinteraction (Variables|Default|GetWidgetInteraction))
  (switch Utilities|FlowControl|Switch|SwitchonEControllerHand (Variables|Default|GetHand)
    (:Left
      (Variables|/Script/UMG.WidgetInteractionComponent|SetPointerIndex _widgetinteraction 0))
    (:Right
      (Variables|/Script/UMG.WidgetInteractionComponent|SetPointerIndex _widgetinteraction 1))))

(fn ConstructionScript
  (bind _returnvalue (CallFunction|GetOculusHandType))
  (bind _oculushand (Variables|Default|GetOculusHand))
  (Variables|/Script/HeadMountedDisplay.MotionControllerComponent|SetMotionSource (Variables|Default|GetMotionController) (Utilities|Name|EnumtoName (Variables|Default|GetHand)))
  (Variables|/Script/OculusInput.OculusHandComponent|SetMeshType _oculushand _returnvalue)
  (Variables|/Script/OculusInput.OculusHandComponent|SetSkeletonType _oculushand _returnvalue))

(fn GetOculusHandType
  (return (Utilities|Select :Index (Variables|Default|GetHand) :Left "HandLeft" :Right "HandRight" :AnyHand "None" :Pad "None" :ExternalCamera "None" :Gun "None" :Special_1 "None" :Special_2 "None" :Special_3 "None" :Special_4 "None" :Special_5 "None" :Special_6 "None" :Special_7 "None" :Special_8 "None" :Special_9 "None" :Special_10 "None" :Special_11 "None")))

(fn UpdateSplineMesh
  (bind _spline (Variables|Default|GetSpline))
  (bind _spline_2 (Variables|Default|GetSpline))
  (bind (_location _tangent) (Spline|GetLocationandTangentatSplinePoint _spline 1 "Local"))
  (bind (_location_2 _tangent_2) (Spline|GetLocationandTangentatSplinePoint _spline_2 0 "Local"))
  (SplineMesh|SetStartandEnd (Variables|Default|GetSplineMesh) _location_2 _tangent_2 _location _tangent true :!class /Script/Engine.SplineMeshComponent))

(fn CollapseSpline
  (Spline|SetLocationatSplinePoint (Variables|Default|GetSpline) 1 (Spline|GetLocationatSplinePoint (Variables|Default|GetSpline) 0 "World") "World" true)
  (CallFunction|UpdateSplineMesh))