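; VR player actor that provides two hands and a toggleable menu.
; On BeginPlay it sets a floor tracking origin, then spawns and attaches left and right BP_Hand actors, which receive index-pinch press and release inputs.
; Releasing Menu input destroys the existing BP_Menu or spawns one using GetMenuTransform.
; That graph holds math for placement 100 units along the camera's flattened forward vector, facing the camera, though it appears unconnected.
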(event EventBeginPlay
  (bind _returnvalue (Math|Transform|MakeTransform "0, 0, 0"))
  (bind _self self)
  (bind _self_2 self)
  (Utilities|FlowControl|Sequence
    (:then_0
      (Class|HeadMountedDisplayFunctionLibrary|SetTrackingOrigin "Floor"))
    (:then_1
      (Utilities|FlowControl|Sequence
        (:then_0
          (bind _returnvalue_2 (Game|SpawnActorfromClass "/Game/BP_Hand.BP_Hand_C" _returnvalue "AlwaysSpawn" _self_2 "Left" 0))
          (bind _output_get (Variables|Default|SetLeft _returnvalue_2))
          (Transformation|AttachActorToActor _output_get _self "None" "SnapToTarget" "SnapToTarget" "KeepWorld" false))
        (:then_1
          (bind _returnvalue_3 (Game|SpawnActorfromClass "/Game/BP_Hand.BP_Hand_C" _returnvalue "AlwaysSpawn" _self_2 "Right" 0))
          (bind _output_get_2 (Variables|Default|SetRight _returnvalue_3))
          (Transformation|AttachActorToActor _output_get_2 _self "None" "SnapToTarget" "SnapToTarget" "KeepWorld" false))))))

(event Input|ActionEvents|InputActionLeftIndexPinch
  (params (Key :type Key%20Structure))
  (bind _left (Variables|Default|GetLeft))
  (:Pressed
    (Default|Press _left))
  (:Released
    (Default|Release _left)))

(event Input|ActionEvents|InputActionRightIndexPinch
  (params (Key :type Key%20Structure))
  (bind _right (Variables|Default|GetRight))
  (:Pressed
    (Default|Press _right))
  (:Released
    (Default|Release _right)))

(event Input|ActionEvents|InputActionMenu
  (params (Key :type Key%20Structure))
  (:Released
    (bind _menu (Variables|Default|GetMenu)
      (:then
        (Actor|DestroyActor _menu))
      (:else
        (bind _returnvalue (Game|SpawnActorfromClass "/Game/BP_Menu.BP_Menu_C" (|GetMenuTransform) "Undefined" 0 0))
        (Variables|Default|SetMenu _returnvalue)))))

(fn ConstructionScript)